(event `self.ReceiveBeginPlay`
  (bind (_settings_buildingtime _settings_buildingmaxresource) (break `/Game/SettingsStruct` (`self.Settings`)))
  ;[1 1 1] Begin Play
  (set `self.BuildTime` _settings_buildingtime)
  (set `self.MaxResource` _settings_buildingmaxresource)
  (bind _asw_progress_bar (cast `/Game/Widgets/W_ProgressBar` (`WidgetComponent.GetUserWidgetObject` (`self.Widget`))))
  (bind _returnvalue (`Image.GetDynamicMaterial` (`/Game/Widgets/W_ProgressBar.ImagePB` _asw_progress_bar)))
  (set `self.WidgetMaterial` _returnvalue)
  (`TextBlock.SetText` (`/Game/Widgets/W_ProgressBar.ResourceText` _asw_progress_bar) (`KismetTextLibrary.Conv_DoubleToText` (`self.MaxResource`) "HalfToEven"))
  (bind _returnvalue_2 (`MaterialInstanceDynamic.K2_GetVectorParameterValue` (`self.WidgetMaterial`) "Color"))
  (set `self.WidgetColor` _returnvalue_2))

(event `self.Box.OnComponentBeginOverlap`
  (params (OverlappedComponent :type "PrimitiveComponent Object Reference") (OtherActor :type "Actor Object Reference") (OtherComp :type "PrimitiveComponent Object Reference") (OtherBodyIndex :type Integer) (bFromSweep :type Boolean) (SweepResult :type "HitResult Structure (by ref)"))
  ;[1 1 1] Overlap stuff - can or can not build there
  (if (`self.IsGhost`)
    (`MaterialInstanceDynamic.SetVectorParameterValue` (`self.Material`) "Color" (struct :`R` 1.0 :`A` 1.0))
    (set `self.CanBuild` false)))

(event `self.Box.OnComponentEndOverlap`
  (params (OverlappedComponent :type "PrimitiveComponent Object Reference") (OtherActor :type "Actor Object Reference") (OtherComp :type "PrimitiveComponent Object Reference") (OtherBodyIndex :type Integer))
  ;[1 1 1] Overlap stuff - can or can not build there
  (if (`self.IsGhost`)
    (`MaterialInstanceDynamic.SetVectorParameterValue` (`self.Material`) "Color" (`self.MainColor`))
    (set `self.CanBuild` true)))

(event `Build`
  (bind _buildtime (`self.BuildTime`))
  ;[1 1 1] Build start and progress
  (set `self.IsGhost` false)
  (`MaterialInstanceDynamic.SetScalarParameterValue` (`self.Material`) "Opacity" 1.0)
  (`SceneComponent.SetHiddenInGame` (`self.Widget`) false false)
  (`PrimitiveComponent.SetCollisionObjectType` (`self.Box`) "ECC_WorldDynamic")
  (`TimelineComponent.SetPlayRate` (`self.BuildingTimeline`) (/ 1.0 (select `bool` (<= _buildtime 0.0) :`false` _buildtime :`true` 0.01)))
  (bind (_direction _time) (`Timeline|BuildingTimeline` :!via `PlayFromStart`)
    (:`Update`
      (`MaterialInstanceDynamic.SetScalarParameterValue` (`self.WidgetMaterial`) "AlphaOut" _time))
    (:`Finished`
      (set `self.IsBuilt` true))))

(event `self.ReceiveTick`
  (params (DeltaSeconds :type "Float (single-precision)"))
  ;[1 1 1] Event Tick
  (if (`self.IsBuilt`)
    (if (< (`self.Resource`) (`self.MaxResource`))
      (bind _output_get (set `self.Resource` (`KismetMathLibrary.FClamp` (+ (* DeltaSeconds 1.0) (`self.Resource`)) 0.0 (`self.MaxResource`))))
      (`MaterialInstanceDynamic.SetScalarParameterValue` (`self.WidgetMaterial`) "AlphaIn" (`KismetMathLibrary.MapRangeClamped` _output_get 0.0 (`self.MaxResource`) 0.0 1.0))
      (if (>= (`self.Resource`) (`self.MaxResource`))
        (`MaterialInstanceDynamic.SetVectorParameterValue` (`self.WidgetMaterial`) "Color" (struct :`R` 1.0 :`A` 1.0))
        (else
          (`MaterialInstanceDynamic.SetVectorParameterValue` (`self.WidgetMaterial`) "Color" (`self.WidgetColor`)))))
    (else
      (`self.SetColorIfResourcesLow`))))

(fn `CollectResources`
  (returns (Resources :type "Float (double-precision)"))
  (locals (AvailableResources :type "Float (double-precision)" :default 0.0))
  (set `local.AvailableResources` (`self.Resource`))
  (set `self.Resource` 0.0)
  (return (`local.AvailableResources`)))

(fn `SetColorIfResourcesLow`
  (if (`self.IsGhost`)
    (if (< (`self.PlayerResources`) (`self.BuildCost`))
      (`MaterialInstanceDynamic.SetVectorParameterValue` (`self.Material`) "Color" (struct :`R` 1.0 :`A` 1.0))
      (elif (`self.CanBuild`)
        (`MaterialInstanceDynamic.SetVectorParameterValue` (`self.Material`) "Color" (`self.MainColor`))))))

(fn `UserConstructionScript`
  (bind _cube (`self.Cube`))
  (bind _returnvalue (`PrimitiveComponent.CreateDynamicMaterialInstance` _cube 0 (`PrimitiveComponent.GetMaterial` _cube 0) "None"))
  (bind _output_get (set `self.Material` _returnvalue))
  (bind _returnvalue_2 (`MaterialInstanceDynamic.K2_GetVectorParameterValue` _output_get "Color"))
  (set `self.MainColor` _returnvalue_2))